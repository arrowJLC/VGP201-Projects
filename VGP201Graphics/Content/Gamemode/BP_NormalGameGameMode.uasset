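; Game mode for the normal game, handling the play timer, checkpoint respawns and game over.
; BeginPlay creates the game-scene HUD and, unless the player's pause-timer flag is set, starts a looping one-second timer that feeds minutes and seconds to it.
; RespawnPlayer moves the player to the last checkpoint and reports a death.
; Three deaths inside a ten-second window show the game-over widget, pause the game and destroy the player.
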(event Custom|RespawnPlayer
  (Transformation|SetActorLocation (Game|GetPlayerCharacter 0) (.location (Transformation|GetWorldTransform (Variables|/Game/BluePrints/BP_CheckPoint.BP_CheckPoint_C|GetPos (Variables|Default|GetlastCheckPoint)))) false false)
  (Input|EnableInput (Variables|Default|GetPlayer) (Game|GetPlayerController 0))
  (CallFunction|ReportPlayerDeath))

(event Custom|ReportPlayerDeath
  (if (Variables|Default|GetisDeathwindowActive)
    (Variables|Default|SetDeathCount (+ (Variables|Default|GetDeathCount) 1))
    (if (>= (Variables|Default|GetDeathCount) 3)
      (Utilities|Time|ClearTimerbyFunctionName 0 "ResetDeathWindow")
      (CallFunction|CallEndGame))
    (else
      (Variables|Default|SetisDeathwindowActive true)
      (Variables|Default|SetDeathCount (+ (Variables|Default|GetDeathCount) 1))
      (Utilities|Time|SetTimerbyFunctionName 0 "ResetDeathWindow" 1e+01 true))))

(event Custom|CallEndGame
  (bind _returnvalue (UserInterface|CreateWidget "/Game/BluePrints/GUI/gameOver/WBP_GameOver.WBP_GameOver_C"))
  (UserInterface|Viewport|AddtoViewport _returnvalue 0)
  (Game|SetGamePaused true)
  (Actor|DestroyActor (Game|GetPlayerCharacter 0)))

(event EventTick
  (params (DeltaSeconds :type Float%20%28single-precision%29))
  (bind _asbp_temp_player (Utilities|Casting|CastToBP_TempPlayer (Game|GetPlayerCharacter 0)))
  (Variables|Default|SetPlayer _asbp_temp_player))

(event EventBeginPlay
  (bind _returnvalue (UserInterface|CreateWidget "/Game/BluePrints/GUI/gameMenu/WPB_GameScene.WPB_GameScene_C"))
  (Variables|Default|SetGameSceneHUD _returnvalue)
  (if (Variables|/Game/playerCharacter/Player/BP_TempPlayer.BP_TempPlayer_C|GetpasueTimer (Variables|Default|GetPlayer))
    (Default|Timer (Variables|Default|GetGameSceneHUD))
    (else
      (Utilities|Time|SetTimerbyFunctionName 0 "Game Timer" 1.0 true)
      (Development|PrintString "Creating Normal GameMode" true true "(R=0.984375,G=0.000000,B=0.080050,A=1.000000)" 5.0)
      (Input|SetInputModeGameOnly (Game|GetPlayerController 0) false))))

(fn ConstructionScript)

(fn GameTimer
  (Math|Integer|IncrementInt (Variables|Default|GetSeconds)
    (:%20%20
      (if (>= (Variables|Default|GetSeconds) 60)
        (bind _output_get (Variables|Default|SetSeconds 0))
        (bind _result (Math|Integer|IncrementInt (Variables|Default|GetMin)))
        (else
          (Default|GameTimer (Variables|Default|GetGameSceneHUD) (Variables|Default|GetSeconds) (Variables|Default|GetMin)))))))

(fn ResetDeathWindow
  (Variables|Default|SetisDeathwindowActive false)
  (Variables|Default|SetDeathCount 0))