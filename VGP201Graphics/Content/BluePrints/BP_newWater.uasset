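; BP_newWater is a moving water hazard that opens a level when BP_TempPlayer hits it.
; The construction script gives InterpToMovement two relative control points, the origin and a Movement offset, timed by Duration.
; A custom event with a component-overlap signature casts to the player, prints a debug message and opens the level; its binding is absent from the graph.
; The ActorBeginOverlap handler only performs the cast.
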(event Custom|CustomEvent
  (params (OverlappedComponent :type Primitive%20Component%20Object%20Reference) (OtherActor :type Actor%20Object%20Reference) (OtherComp :type Primitive%20Component%20Object%20Reference) (OtherBodyIndex :type Integer) (bFromSweep :type Boolean) (SweepResult :type Hit%20Result%20Structure%20%28by%20ref%29))
  (Utilities|Casting|CastToBP_TempPlayer OtherActor)
  (Development|PrintString "Player hit water")
  (Game|OpenLevel(byObjectReference)))

(event EventBeginPlay)

(event Collision|EventActorBeginOverlap
  (params (OtherActor :type Actor%20Object%20Reference))
  (Utilities|Casting|CastToBP_TempPlayer OtherActor))

(event EventTick
  (params (DeltaSeconds :type Float%20%28single-precision%29)))

(fn ConstructionScript
  (bind _interptomovement (Variables|Default|GetInterpToMovement))
  (Class|InterptoMovementComponent|AddControlPointPosition _interptomovement "0, 0, 0" true)
  (Class|InterptoMovementComponent|AddControlPointPosition (Variables|Default|GetInterpToMovement) (Variables|Default|GetMovement) true)
  (Variables|/Script/Engine.InterpToMovementComponent|SetDuration _interptomovement (Variables|Default|GetDuration)))