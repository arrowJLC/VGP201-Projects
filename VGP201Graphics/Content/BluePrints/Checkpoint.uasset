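; Checkpoint trigger actor that starts the rising-water phase when the player reaches it.
; On BeginPlay it finds the first BP_waterLevels actor in the level and caches it.
; When the player pawn overlaps it, it prints checkpoint and water-rise messages and sets that actor's HitCheck flag to true.
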(event EventBeginPlay
  (bind _outactors (Actor|GetAllActorsOfClass "/Game/BluePrints/BP_waterLevels.BP_waterLevels_C"))
  (Variables|Default|SetNewVar (Utilities|Array|Get(acopy) _outactors)))

(event Collision|EventActorBeginOverlap
  (params (OtherActor :type Actor%20Object%20Reference))
  (if (== OtherActor (Game|Player|GetPlayerPawn 0))
    (Development|PrintString "Checkpoint")
    (Development|PrintString "Water Will Start To Rise")
    (Variables|/Game/BluePrints/BP_waterLevels.BP_waterLevels_C|SethitCheck (Variables|Default|GetNewVar) true)))

(fn ConstructionScript)